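; BP_ObjetTest is a test object that highlights itself when the player can pick it up.
; HighlightObject raises the point light's intensity, enables custom depth on the cube and shows the hint text on the first-person character's HUD.
; Tick undoes all three every frame, so the highlight only holds while HighlightObject is called repeatedly.
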(event Custom|HighlightObject
  ;[1 1 1] Allumer lumière objet quand ramassable par le joueur
  (Rendering|Components|Light|SetIntensity (Variables|Default|GetPointLight) 5e+03)
  ;[1 1 1] Afficher le texte
  (bind _asfirst_person_character (Utilities|Casting|CastToFirstPersonCharacter (Game|GetPlayerCharacter 0)))
  (Default|ToggleHintText (Variables|/Game/FirstPersonBP/Blueprints/FirstPersonCharacter.FirstPersonCharacter_C|GetHUD_MainRef _asfirst_person_character) true)
  (Rendering|SetRenderCustomDepth (Variables|Default|GetCube) true))

(event EventTick
  (params (DeltaSeconds :type Float%20%28single-precision%29))
  ;[1 1 1] Eteindre la lumière de l'objet
  (Rendering|Components|Light|SetIntensity (Variables|Default|GetPointLight) 0.0)
  ;[1 1 1] Cacher le texte
  (bind _asfirst_person_character (Utilities|Casting|CastToFirstPersonCharacter (Game|GetPlayerCharacter 0)))
  (Default|ToggleHintText (Variables|/Game/FirstPersonBP/Blueprints/FirstPersonCharacter.FirstPersonCharacter_C|GetHUD_MainRef _asfirst_person_character) false)
  (Rendering|SetRenderCustomDepth (Variables|Default|GetCube) false))

(fn ConstructionScript)